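; BP_Player is a player Blueprint that briefly flashes its mesh color when the Fire action is used.
; BeginPlay stores a base and an event color, then binds OnFireEvent to the Fire action.
; OnFireEvent writes the event color to the Color parameter on the StaticMesh materials, then restores the base color after a short Delay.
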(event `self.ReceiveBeginPlay`
  ;[1 1 1] Sets the default and even colors
  (set `self.Base_Color_Vector` (0.25 0.15 0.25))
  (set `self.Event_Color_Vector` (0.1 0.05 0.1))
  (add `self.OnFireAction` (delegate `OnFireEvent`)))

(event `OnFireEvent`
  ;[1 1 1] When Player uses the Fire Action the color briefly changes, and then changes back.
  (`MeshComponent.SetVectorParameterValueOnMaterials` (`self.StaticMesh`) "Color" (`self.Event_Color_Vector`))
  (`KismetSystemLibrary.Delay` 0.1)
  (`MeshComponent.SetVectorParameterValueOnMaterials` (`self.StaticMesh`) "Color" (`self.Base_Color_Vector`)))

(fn `UserConstructionScript`)